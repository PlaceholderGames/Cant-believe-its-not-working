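; Keypad terminal actor that stays unpowered until unlocked, then lets the player open a code-entry widget.
; Unlocking powers it, generates a random four-digit password and messages it to actors tagged PasswordSet.
; Interact creates the KeypadWidget on first use, shows it and passes it the password, or prints "No Power" when unpowered.
; CorrectPassword switches the cube's material to a green light.
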(event EventInteract
  (if (Variables|Default|GetPowered)
    (if (Variables|Default|GetWidgetCreated)
      (Widget|GetAllWidgetsOfClass "/Game/Objects/Terminals/Keypad/KeypadWidget.KeypadWidget_C" false)
      (else
        (bind _returnvalue (UserInterface|CreateWidget "/Game/Objects/Terminals/Keypad/KeypadWidget.KeypadWidget_C"))
        (Variables|Default|SetWidgetCreated true)))
    (UserInterface|Viewport|AddtoPlayerScreen _returnvalue)
    (Class|CharacterInteraction|PasswordSet(Message) _returnvalue (Utilities|Text|ToText(String) (Variables|Default|GetRandomPasswordString)))
    (else
      (Development|PrintString "No Power"))))

(event EventCorrectPassword
  (Rendering|Material|SetMaterial (Variables|Default|GetCube) 0 "/Game/Geometry/Materials/GreenLight.GreenLight"))

(event EventUnlocking
  (Variables|Default|SetPowered true)
  (CallFunction|RandomPassword)
  (bind _outactors (Actor|GetAllActorswithTag "PasswordSet"))
  (Class|CharacterInteraction|PasswordSet(Message) _outactors (Utilities|Text|ToText(String) (Variables|Default|GetRandomPasswordString))))

(fn ConstructionScript)

(fn RandomPassword
  (for _index (range 0 3)
    (Variables|Default|SetRandomPasswordString (Utilities|String|Append (Variables|Default|GetRandomPasswordString) (Utilities|String|ToString(Integer) (Math|Random|RandomIntegerinRange 0 9))))))