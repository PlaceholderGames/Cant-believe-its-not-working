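; GameTerminalBP is an interactable terminal that opens a HackSlider hacking widget and pauses the game.
; Interaction requires Powered, set by the Unlocking event; otherwise it prints "No Power".
; The first use creates the widget and passes it the password received through PasswordSet.
; Later uses re-add the stored widget to the player screen, after a GetAllWidgetsOfClass call whose result is unused.
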(event EventPasswordSet
  (params (Password :type Text))
  (Variables|Default|SetCorrectPasswordText Password))

(event EventInteract
  (if (Variables|Default|GetPowered)
    (if (Variables|Default|GetWidgetCreated)
      (Widget|GetAllWidgetsOfClass "/Game/Objects/Terminals/GameTerminal/HackSlider.HackSlider_C" true)
      (else
        (bind _returnvalue (UserInterface|CreateWidget "/Game/Objects/Terminals/GameTerminal/HackSlider.HackSlider_C"))
        (Variables|Default|SetWidgetCreated true)
        (Class|CharacterInteraction|PasswordSet(Message) _returnvalue (Variables|Default|GetCorrectPasswordText))))
    (UserInterface|Viewport|AddtoPlayerScreen _returnvalue)
    (Game|SetGamePaused true)
    (else
      (Development|PrintString "No Power"))))

(event EventUnlocking
  (Variables|Default|SetPowered true))

(fn ConstructionScript)