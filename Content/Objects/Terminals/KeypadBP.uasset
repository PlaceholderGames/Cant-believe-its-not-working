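; Keypad Blueprint that generates a random numeric code when unlocked and shows a keypad UI when interacted with.
; The Unlocking event powers it, builds a four-digit string and sends it to every GameTerminalBP actor through PasswordMessage.
; Once powered, Interact creates a KeypadWidget on first use, adds it to the player screen and passes it the same code.
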(event EventInteract
  (if (Variables|Default|GetPowered)
    (if (Variables|Default|GetWidgetCreated)
      (Widget|GetAllWidgetsOfClass "/Game/Objects/Terminals/KeypadWidget.KeypadWidget_C" false)
      (else
        (bind _returnvalue (UserInterface|CreateWidget "/Game/Objects/Terminals/KeypadWidget.KeypadWidget_C"))
        (Variables|Default|SetWidgetCreated true)))
    (UserInterface|Viewport|AddtoPlayerScreen _returnvalue)
    (Class|CharacterInteraction|Password(Message) _returnvalue (Utilities|Text|ToText(String) (Variables|Default|GetRandomPassword)))))

(event EventUnlocking
  (Variables|Default|SetPowered true)
  (CallFunction|RandomPassword)
  (bind _outactors (Actor|GetAllActorsOfClass "/Game/Objects/Terminals/GameTerminalBP.GameTerminalBP_C"))
  (Class|CharacterInteraction|Password(Message) _outactors (Utilities|Text|ToText(String) (Variables|Default|GetRandomPassword))))

(fn ConstructionScript)

(fn RandomPassword
  (for _index (range 0 3)
    (Variables|Default|SetRandomPassword (Utilities|String|Append (Variables|Default|GetRandomPassword) (Utilities|String|ToString(Integer) (Math|Random|RandomIntegerinRange 0 9))))))