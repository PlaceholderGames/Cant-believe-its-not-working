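; Keypanel Blueprint for a keycard reader that opens the nearest door when the player holds the first keycard.
; On Interact, it casts the player character to CharacterBP and checks the KeyCardOneInInventory flag.
; If the flag is set, it destroys the door returned by FindNearestDoor, switches the Cube to the GreenLight material and sets Used to block further activation.
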(event EventInteract
  (if (not (Variables|Default|GetUsed))
    (bind _ascharacter_bp (Utilities|Casting|CastToCharacterBP (Game|GetPlayerCharacter 0)))
    (if (Variables|/Game/CharacterBP/CharacterBP.CharacterBP_C|GetKeyCardOneInInventory _ascharacter_bp)
      (bind _closest (CallFunction|FindNearestDoor self))
      (Actor|DestroyActor _closest)
      (Variables|Default|SetUsed true)
      (Rendering|Material|SetMaterial (Variables|Default|GetCube) 0 "/Game/Geometry/Materials/GreenLight.GreenLight"))))

(fn ConstructionScript)